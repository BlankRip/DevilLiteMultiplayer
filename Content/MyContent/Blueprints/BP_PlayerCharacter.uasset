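; BP_PlayerCharacter is a player character Blueprint with debug key bindings for testing the GA_RapidArrowTest gameplay ability.
; Number keys grant the ability through the Ability System, clear it, and try to activate it, allowing remote activation.
; The spec handle from the grant is kept in TestAbilitySlot for clearing and activation, and is reset on removal.
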(event `Key|One`
  (params (Key :type "Key Structure"))
  (:`Pressed`
    (bind _returnvalue (`AbilitySystemComponent.K2_GiveAbility` (`self.AbilitySystem`) "/Game/MyContent/Blueprints/TestingBps/GA_RapidArrowTest.GA_RapidArrowTest_C" 0 -1))
    (set `self.TestAbilitySlot` _returnvalue)))

(event `Key|Two`
  (params (Key :type "Key Structure"))
  (:`Pressed`
    (`AbilitySystemComponent.ClearAbility` (`self.AbilitySystem`) (`self.TestAbilitySlot`))
    (set `self.TestAbilitySlot` (struct))))

(event `Key|Three`
  (params (Key :type "Key Structure"))
  (:`Pressed`
    (`AbilitySystemComponent.TryActivateAbility` (`self.AbilitySystem`) (`self.TestAbilitySlot`) true)))

(event `Key|Four`
  (params (Key :type "Key Structure")))

(fn `UserConstructionScript`)